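; Actor Blueprint that recreates a Blender curve as a spline from a CSV-imported Data Table, optionally lining it with deformed meshes.
; GenerateSplineFromBlender reads positions, tangents and tilt per row, caching them in SavedSplinePointsData.
; The construction script rebuilds the spline from that cache, so manual point edits do not persist.
; It then places SplineMeshComponents at mesh-length intervals, matching spline roll and clamping tangents to segment length.
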(event Custom|Generate%20Spline%20From%20Blender
  (bind _spline (Variables|Default|GetSpline))
  (bind _spline_data_table (Variables|Default|GetSpline%20Data%20Table))
  ;[1 1 1] Generate Spline from Data Table (CSV) - Spline will not be modifiable after it has been generated.
  (Utilities|Array|Clear (Variables|Default|GetSavedSplinePointsData))
  (Spline|ClearSplinePoints (Variables|Default|GetSpline) true)
  (bind _outrownames (DataTable|GetDataTableRowNames _spline_data_table))
  (for (_array_element _array_index) _outrownames
    (bind _returnvalue (Utilities|GetDataTableRow _spline_data_table _array_element)
      (:then
        (Spline|AddSplinePoint _spline (Math|Vector|MakeVector (.XPos (Utilities|Struct|BreakSTR_BlenderCurveData _returnvalue)) (.YPos (Utilities|Struct|BreakSTR_BlenderCurveData _returnvalue)) (.ZPos (Utilities|Struct|BreakSTR_BlenderCurveData _returnvalue))) "Local" false)
        (Spline|SetTangentsatSplinePoint _spline _array_index (Math|Vector|MakeVector (.XHandleIn (Utilities|Struct|BreakSTR_BlenderCurveData _returnvalue)) (.YHandleIn (Utilities|Struct|BreakSTR_BlenderCurveData _returnvalue)) (.ZHandleIn (Utilities|Struct|BreakSTR_BlenderCurveData _returnvalue))) (Math|Vector|MakeVector (.XHandleOut (Utilities|Struct|BreakSTR_BlenderCurveData _returnvalue)) (.YHandleOut (Utilities|Struct|BreakSTR_BlenderCurveData _returnvalue)) (.ZHandleOut (Utilities|Struct|BreakSTR_BlenderCurveData _returnvalue))) "Local" false)
        (Spline|SetRotationatSplinePoint _spline _array_index (Math|Rotator|MakeRotator (.Tilt (Utilities|Struct|BreakSTR_BlenderCurveData _returnvalue)) (.pitch (Spline|GetRotationatSplinePoint _spline _array_index "Local")) (.yaw (Spline|GetRotationatSplinePoint _spline _array_index "Local"))) "Local" false)
        (Spline|SetSplinePointType _spline _array_index "Curve" false)
        ;[1 1 1] Save Spline Points Data after being Generated
        (Utilities|Array|Add (Variables|Default|GetSavedSplinePointsData) (Utilities|Struct|MakeSTR_SplinePointsData (Math|Vector|MakeVector (.XPos (Utilities|Struct|BreakSTR_BlenderCurveData _returnvalue)) (.YPos (Utilities|Struct|BreakSTR_BlenderCurveData _returnvalue)) (.ZPos (Utilities|Struct|BreakSTR_BlenderCurveData _returnvalue))) (Math|Vector|MakeVector (.XHandleIn (Utilities|Struct|BreakSTR_BlenderCurveData _returnvalue)) (.YHandleIn (Utilities|Struct|BreakSTR_BlenderCurveData _returnvalue)) (.ZHandleIn (Utilities|Struct|BreakSTR_BlenderCurveData _returnvalue))) (Math|Vector|MakeVector (.XHandleOut (Utilities|Struct|BreakSTR_BlenderCurveData _returnvalue)) (.YHandleOut (Utilities|Struct|BreakSTR_BlenderCurveData _returnvalue)) (.ZHandleOut (Utilities|Struct|BreakSTR_BlenderCurveData _returnvalue))) "Curve" (Math|Rotator|MakeRotator (.Tilt (Utilities|Struct|BreakSTR_BlenderCurveData _returnvalue)) (.pitch (Spline|GetRotationatSplinePoint _spline _array_index "Local")) (.yaw (Spline|GetRotationatSplinePoint _spline _array_index "Local"))))))))
  (Spline|UpdateSpline _spline))

(fn ConstructionScript
  (bind _spline (Variables|Default|GetSpline))
  (Utilities|FlowControl|Sequence
    (:then_0
      ;[1 1 1] Rebuild Spline After Blueprint Moved in the Viewport
      (if (> (Utilities|Array|Length (Variables|Default|GetSavedSplinePointsData)) 0)
        (CallFunction|RebuildSplinefromSavedPoints)))
    (:then_1
      ;[1 1 1] Add Mesh Along Spline (this part is based on SplineTools by tiedtke (available on Gumroad) with some improvements for use with a generated spline.).
      (if (Variables|AddMeshAlongSpline|GetAdd%20Mesh%20Along%20Spline?)
        (Variables|AddMeshAlongSpline|SetMesh%20X%20Length (* (.x (.boxextent (StaticMesh|GetBounds (Variables|AddMeshAlongSpline|GetMesh)))) 2.0))
        (for _index (range 0 (Math|Float|Truncate (/ (Spline|GetSplineLength (Variables|Default|GetSpline)) (Variables|AddMeshAlongSpline|GetMesh%20X%20Length))))
          ;;[1 1 1] Mesh
          (bind _returnvalue (AddComponent|AddSplineMeshComponent false))
          (Collision|SetActorEnableCollision (Variables|AddMeshAlongSpline|GetCollision?))
          (Components|StaticMesh|SetStaticMesh _returnvalue (Variables|AddMeshAlongSpline|GetMesh))
          (SplineMesh|SetForwardAxis _returnvalue "X" true)
          (SplineMesh|SetStartRollDegrees _returnvalue (Class|SplineComponent|GetRollatDistanceAlongSpline _spline (* _index (Variables|AddMeshAlongSpline|GetMesh%20X%20Length)) "Local") true)
          (SplineMesh|SetEndRollDegrees _returnvalue (Class|SplineComponent|GetRollatDistanceAlongSpline _spline (* (+ _index 1) (Variables|AddMeshAlongSpline|GetMesh%20X%20Length)) "Local") true)
          (SplineMesh|SetStartandEnd _returnvalue (Spline|GetLocationatDistanceAlongSpline _spline (* _index (Variables|AddMeshAlongSpline|GetMesh%20X%20Length)) "Local") (Math|Vector|ClampVectorSize (Spline|GetTangentatDistanceAlongSpline _spline (* _index (Variables|AddMeshAlongSpline|GetMesh%20X%20Length)) "Local") 0.0 (Variables|AddMeshAlongSpline|GetMesh%20X%20Length)) (Spline|GetLocationatDistanceAlongSpline _spline (* (+ _index 1) (Variables|AddMeshAlongSpline|GetMesh%20X%20Length)) "Local") (Math|Vector|ClampVectorSize (Spline|GetTangentatDistanceAlongSpline _spline (* (+ _index 1) (Variables|AddMeshAlongSpline|GetMesh%20X%20Length)) "Local") 0.0 (Variables|AddMeshAlongSpline|GetMesh%20X%20Length)) true :!class /Script/Engine.SplineMeshComponent))))))

(fn RebuildSplinefromSavedPoints
  (bind _spline (Variables|Default|GetSpline))
  ;[1 1 1] Rebuild Spline from Saved Points
  (Spline|ClearSplinePoints (Variables|Default|GetSpline) true)
  (for (_array_element _array_index) (Variables|Default|GetSavedSplinePointsData)
    (Spline|AddSplinePoint _spline (.position _array_element) "Local" false)
    (Spline|SetTangentsatSplinePoint _spline _array_index (.intangent _array_element) (.outtangent _array_element) "Local" false)
    (Spline|SetRotationatSplinePoint _spline _array_index (.rotation _array_element) "Local" false)
    (Spline|SetSplinePointType _spline _array_index (.splinepointtype _array_element) false))
  (Spline|UpdateSpline (Variables|Default|GetSpline)))