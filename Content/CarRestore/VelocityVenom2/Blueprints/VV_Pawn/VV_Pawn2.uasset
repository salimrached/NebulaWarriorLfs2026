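; Player vehicle pawn for a physics-driven car with boost, chase-camera look and speed HUD.
; Enhanced Input applies forces and torque to the box body, with downforce on sphere wheels; boost multiplies acceleration and triggers exhaust particles and sound.
; Tick syncs wheel meshes to spheres, clamps pitch and roll, and updates the HUD.
; Forward speed also selects one of six simulated gears, using DoOnce gates to retrigger the MetaSound engine audio.
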(event Custom|getCurrentGear
  (if (Math|Integer|InRange(Integer) (CallFunction|GetSpeed) -300 9)
    (Variables|Default|Setgear 0)
    (Utilities|FlowControl|DoOnce false
      (:Completed
        (CallFunction|ResetGear)
        (CallFunction|ResetGear2)
        (CallFunction|ResetGear3)
        (CallFunction|ResetGear4)
        (CallFunction|ResetGear5)
        (CallFunction|ChangeGear)
        (CallFunction|ChangeGear :!label _label)))
    (elif (Math|Integer|InRange(Integer) (CallFunction|GetSpeed) 10 20)
      (Variables|Default|Setgear 1)
      (Utilities|FlowControl|DoOnce false
        (:Completed
          (CallFunction|ResetGear)
          (CallFunction|ResetGear1)
          (CallFunction|ResetGear3)
          (CallFunction|ResetGear4)
          (CallFunction|ResetGear5)
          (CallFunction|ResetGear6)
          (goto _label)))
      (elif (Math|Integer|InRange(Integer) (CallFunction|GetSpeed) 21 30)
        (Variables|Default|Setgear 2)
        (Utilities|FlowControl|DoOnce false
          (:Completed
            (CallFunction|ResetGear)
            (CallFunction|ResetGear1)
            (CallFunction|ResetGear2)
            (CallFunction|ResetGear4)
            (CallFunction|ResetGear5)
            (CallFunction|ResetGear6)
            (goto _label)))
        (elif (Math|Integer|InRange(Integer) (CallFunction|GetSpeed) 31 60)
          (Variables|Default|Setgear 3)
          (Utilities|FlowControl|DoOnce false
            (:Completed
              (CallFunction|ResetGear)
              (CallFunction|ResetGear1)
              (CallFunction|ResetGear2)
              (CallFunction|ResetGear3)
              (CallFunction|ResetGear5)
              (CallFunction|ResetGear6)
              (CallFunction|ChangeGear)))
          (elif (Math|Integer|InRange(Integer) (CallFunction|GetSpeed) 61 100)
            (Variables|Default|Setgear 4)
            (Utilities|FlowControl|DoOnce false
              (:Completed
                (CallFunction|ResetGear)
                (CallFunction|ResetGear1)
                (CallFunction|ResetGear2)
                (CallFunction|ResetGear3)
                (CallFunction|ResetGear4)
                (CallFunction|ResetGear6)
                (CallFunction|ChangeGear)))
            (elif (> (CallFunction|GetSpeed) 100)
              (Variables|Default|Setgear 5)
              (Utilities|FlowControl|DoOnce false
                (:Completed
                  (CallFunction|ResetGear)
                  (CallFunction|ResetGear1)
                  (CallFunction|ResetGear2)
                  (CallFunction|ResetGear3)
                  (CallFunction|ResetGear4)
                  (CallFunction|ResetGear5)
                  (CallFunction|ChangeGear))))))))))

(event Custom|controlVehicleRotation
  (bind _returnvalue (Transformation|GetActorRotation))
  (Transformation|SetActorRotation (Math|Rotator|MakeRotator (Math|Float|Clamp(Float) (.roll _returnvalue) -3e+01 3e+01) (Math|Float|Clamp(Float) (.pitch _returnvalue) -3e+01 3e+01) (.yaw _returnvalue))))

(event Custom|resetGear4
  (Utilities|FlowControl|DoOnce false) ; enters at Reset
)

(event Custom|resetGear6
  (Utilities|FlowControl|DoOnce false) ; enters at Reset
)

(event Custom|resetGear5
  (Utilities|FlowControl|DoOnce false) ; enters at Reset
)

(event Custom|changeGear
  (Utilities|FlowControl|DoOnce false
    (:Completed
      (Effects|Components|ParticleSystem|SetIntParameter (Variables|Default|GetMS_EngineSound) "Index" (Variables|Default|Getgear))
      (Class|AudioParameterControllerInterface|SetTriggerParameter (Variables|Default|GetMS_EngineSound) "Trigger2")
      (Class|AudioParameterControllerInterface|SetTriggerParameter (Variables|Default|GetMS_EngineSound) "Play")
      (EventDispatchers|AssignOnAudioFinished (Variables|Default|GetMS_EngineSound) (delegate Custom|OnAudioFinished_Event)))))

(event Custom|OnAudioFinished_Event
  (CallFunction|ResetGear))

(event Custom|resetGear1
  (Utilities|FlowControl|DoOnce false) ; enters at Reset
)

(event Custom|resetGear2
  (Utilities|FlowControl|DoOnce false) ; enters at Reset
)

(event Custom|resetGear
  (Utilities|FlowControl|DoOnce false) ; enters at Reset
)

(event Custom|resetGear3
  (Utilities|FlowControl|DoOnce false) ; enters at Reset
)

(event EventBeginPlay
  (CallFunction|Setup))

(event EventTick
  (params (DeltaSeconds :type Float%20%28single-precision%29))
  (CallFunction|WheelsMesh)
  (CallFunction|DisplaySpeedinKmH)
  (CallFunction|ControlVehicleRotation)
  (CallFunction|GetCurrentGear))

(fn ConstructionScript)

(fn GetSpeed
  (return (Math|Float|Round (/ (.X (Math|Vector|BreakVector (Math|Transform|InverseTransformDirection (Transformation|GetActorTransform) (Transformation|GetVelocity)))) 1e+02))))

(event Custom|WheelsMesh
  (bind _staticmesh (Variables|Default|GetStaticMesh))
  (bind _sphere3 (Variables|Default|GetSphere3))
  (bind _staticmesh1 (Variables|Default|GetStaticMesh1))
  (bind _sphere2 (Variables|Default|GetSphere2))
  (bind _staticmesh2 (Variables|Default|GetStaticMesh2))
  (bind _sphere (Variables|Default|GetSphere))
  (bind _staticmesh3 (Variables|Default|GetStaticMesh3))
  (bind _sphere1 (Variables|Default|GetSphere1))
  (Transformation|SetRelativeRotation _staticmesh (Math|Rotator|MakeRotator (.pitch (Variables|/Script/Engine.SceneComponent|GetRelativeRotation _sphere3)) 0.0 9e+01) false false)
  (Transformation|SetWorldLocation _staticmesh (Transformation|GetWorldLocation _sphere3) false false)
  (Transformation|SetRelativeRotation _staticmesh1 (Math|Rotator|MakeRotator (.pitch (Variables|/Script/Engine.SceneComponent|GetRelativeRotation _sphere2)) 0.0 9e+01) false false)
  (Transformation|SetWorldLocation _staticmesh1 (Transformation|GetWorldLocation _sphere2) false false)
  (Transformation|SetRelativeRotation _staticmesh2 (Math|Rotator|MakeRotator (.pitch (Variables|/Script/Engine.SceneComponent|GetRelativeRotation _sphere)) 0.0 9e+01) false false)
  (Transformation|SetWorldLocation _staticmesh2 (Transformation|GetWorldLocation _sphere) false false)
  (Transformation|SetRelativeRotation _staticmesh3 (Math|Rotator|MakeRotator (.pitch (Variables|/Script/Engine.SceneComponent|GetRelativeRotation _sphere1)) 0.0 9e+01) false false)
  (Transformation|SetWorldLocation _staticmesh3 (Transformation|GetWorldLocation _sphere1) false false))

(event Custom|Setup
  (CallFunction|AddMappingInput)
  (CallFunction|AddCarHud)
  (CallFunction|CreateEngineSoundsArray))

(event Custom|addMappingInput
  ;[1 1 1] Add Mapping Input
  (Input|AddMappingContext (PlayerController|LocalPlayerSubsystems|GetEnhancedInputLocalPlayerSubsystem (Game|GetPlayerController 0)) "/Game/CarRestore/VelocityVenom2/Blueprints/VV_Pawn/Input/MC_VVPawn.MC_VVPawn" 0 "(bIgnoreAllPressedKeysUntilRelease=True,bForceImmediately=False,bNotifyUserSettings=False)"))

(event Custom|addCarHud
  ;[1 1 1] addCarHud
  (bind _returnvalue (UserInterface|CreateWidget "/Game/CarRestore/VelocityVenom2/Widgets/General/WB_CarHud.WB_CarHud_C"))
  (bind _output_get (Variables|Default|SetWB_CarHud _returnvalue))
  (UserInterface|Viewport|AddtoViewport _output_get 0))

(event Custom|createEngineSoundsArray
  (bind _enginesounds (Variables|Default|GetEngineSounds))
  (bind (_gear0 _gear1 _gear2 _gear3 _gear4 _gear5) (Utilities|Struct|BreakEngineSoundsArray _enginesounds))
  ;[1 1 1] createEngineSoundsArray
  (Variables|Default|SetSoundsEngineArray (Utilities|Array|MakeArray _gear0 _gear1 _gear2 _gear3 _gear4 _gear5)))

(event Custom|gearChangeSound
  (bind _returnvalue (Audio|CreateSound2D (Utilities|Array|Get(acopy) (Variables|Default|GetSoundsEngineArray) (Variables|Default|Getgear)) 1.0 1.0 0.0 0))
  (Variables|Default|SetcurrentEngineSound _returnvalue))

(event Custom|activateThrustParticles
  ;[1 1 1] IA_Boost
  (Components|Activation|Activate (Variables|Default|GetNS_RocketExhaust_Realistic) false))

(event Custom|DeactivateThrustParticles
  ;[1 1 1] IA_Boost
  (Components|Activation|Deactivate (Variables|Default|GetNS_RocketExhaust_Realistic1)))

(event Custom|soundBoost
  (Utilities|FlowControl|DoOnce false
    (:Completed
      (bind _returnvalue (Audio|CreateSound2D "/Game/CarRestore/VelocityVenom2/Sound/MS_Boost.MS_Boost" 1.0 1.0 0.0 0))
      (Audio|Components|Audio|Play _returnvalue 0.0)
      (EventDispatchers|AssignOnAudioFinished _returnvalue (delegate Custom|OnAudioFinished_Event_0)))))

(event Custom|OnAudioFinished_Event_0
  (Utilities|FlowControl|DoOnce false) ; enters at Reset
)

(event Input|EnhancedActionEvents|EnhancedInputActionIA_Accelerate
  (params (ActionValue :type Boolean) (ElapsedSeconds :type Float%20%28double-precision%29) (TriggeredSeconds :type Float%20%28double-precision%29) (InputAction :type Input%20Action%20Object%20Reference :default "/Game/CarRestore/VelocityVenom2/Blueprints/VV_Pawn/Input/IA_Accelerate.IA_Accelerate"))
  (Physics|AddForce (Variables|Default|GetBox) (* (* (Math|Vector|GetForwardVector (Variables|Default|GetBox)) (Variables|Default|GetAccelerationForce)) (Variables|Default|Getboost)) "None" true)
  (Physics|AddForce (Variables|Default|GetSphere3) "0.000000,0.000000,-600.000000" "None" true))

(event Input|EnhancedActionEvents|EnhancedInputActionIA_Look
  (params (ActionValue :type Vector%202D%20Structure) (ElapsedSeconds :type Float%20%28double-precision%29) (TriggeredSeconds :type Float%20%28double-precision%29) (InputAction :type Input%20Action%20Object%20Reference :default "/Game/CarRestore/VelocityVenom2/Blueprints/VV_Pawn/Input/IA_Look.IA_Look"))
  (bind (_x _y) (Math|Vector2D|BreakVector2D ActionValue))
  ;[1 1 1] IA_Look
  (Transformation|AddRelativeRotation (Variables|Default|GetSpringArm) (Math|Rotator|MakeRotator 0.0 _y _x) false false))

(event Input|EnhancedActionEvents|EnhancedInputActionIA_Boost
  (params (ActionValue :type Boolean) (ElapsedSeconds :type Float%20%28double-precision%29) (TriggeredSeconds :type Float%20%28double-precision%29) (InputAction :type Input%20Action%20Object%20Reference :default "/Game/CarRestore/VelocityVenom2/Blueprints/VV_Pawn/Input/IA_Boost.IA_Boost"))
  ;[1 1 1] IA_Boost
  (:Triggered
    (Variables|Default|Setboost 4.0)
    (Physics|AddForce (Variables|Default|GetBox) "0.000000,0.000000,-300.000000" "None" true)
    (CallFunction|ActivateThrustParticles)
    (CallFunction|SoundBoost))
  (:Completed
    (Variables|Default|Setboost 1.0)
    (CallFunction|DeactivateThrustParticles)))

(event Input|EnhancedActionEvents|EnhancedInputActionIA_Steer
  (params (ActionValue :type Float%20%28double-precision%29) (ElapsedSeconds :type Float%20%28double-precision%29) (TriggeredSeconds :type Float%20%28double-precision%29) (InputAction :type Input%20Action%20Object%20Reference :default "/Game/CarRestore/VelocityVenom2/Blueprints/VV_Pawn/Input/IA_Steer.IA_Steer"))
  (Class|PrimitiveComponent|AddTorqueinRadians (Variables|Default|GetBox) (Math|Vector|MakeVector 0.0 0.0 (* (* ActionValue 3.14) 3.0)) "None" true)
  (Physics|AddForce (Variables|Default|GetBox) (* (* (Math|Vector|GetRightVector (Variables|Default|GetBox)) (Input|EnhancedActionValues|GetIA_Steer)) 1.5e+03) "None" true))

(event Input|EnhancedActionEvents|EnhancedInputActionIA_Break
  (params (ActionValue :type Boolean) (ElapsedSeconds :type Float%20%28double-precision%29) (TriggeredSeconds :type Float%20%28double-precision%29) (InputAction :type Input%20Action%20Object%20Reference :default "/Game/CarRestore/VelocityVenom2/Blueprints/VV_Pawn/Input/IA_Break.IA_Break"))
  (bind _returnvalue (Physics|GetPhysicsLinearVelocity (Variables|Default|GetBox) "None"))
  (Physics|SetPhysicsLinearVelocity (Variables|Default|GetBox) (Math|Interpolation|VInterpTo _returnvalue "0, 0, 0" ElapsedSeconds 0.3) false "None"))

(event Input|KeyboardEvents|E
  (params (Key :type Key%20Structure :default "None"))
  ;[1 1 1] Reset vehicle
)

(event Custom|displaySpeedinKmH
  (Default|UpdateSpeed (Variables|Default|GetWB_CarHud) (Utilities|Text|ToText(Integer) (CallFunction|GetSpeed))))