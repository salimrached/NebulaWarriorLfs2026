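; VV_Pawn1 is a player-driven vehicle pawn that moves by applying physics forces to a Box, with a spring-arm look camera.
; Setup on BeginPlay adds the Enhanced Input mapping context.
; Accelerate pushes forward, scaled by Boost; Break damps velocity, then applies reverse force after a hold; Steer applies yaw torque.
; A temporary key lifts and resets the Box, and several older steering experiments remain disconnected.
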(event Custom|Setup
  (CallFunction|AddMappingInput))

(event Custom|addMappingInput
  ;[1 1 1] Add Mapping Input
  (Input|SetInputModeGameOnly (Game|GetPlayerController 0) false)
  (bind _asplayer_controller (Utilities|Casting|CastToPlayerController (Pawn|GetController)))
  (Utilities|IsValid (PlayerController|LocalPlayerSubsystems|GetEnhancedInputLocalPlayerSubsystem _asplayer_controller)
    (:Is%20Valid
      (Input|AddMappingContext (PlayerController|LocalPlayerSubsystems|GetEnhancedInputLocalPlayerSubsystem _asplayer_controller) "/Game/CarRestore/VelocityVenom2/Blueprints/VV_Pawn/Input/MC_VVPawn.MC_VVPawn" 0 "(bIgnoreAllPressedKeysUntilRelease=True,bForceImmediately=False,bNotifyUserSettings=False)"))))

(event Input|EnhancedActionEvents|EnhancedInputActionIA_Accelerate
  (params (ActionValue :type Boolean) (ElapsedSeconds :type Float%20%28double-precision%29) (TriggeredSeconds :type Float%20%28double-precision%29) (InputAction :type Input%20Action%20Object%20Reference :default "/Game/CarRestore/VelocityVenom2/Blueprints/VV_Pawn/Input/IA_Accelerate.IA_Accelerate"))
  (bind _output_get (Variables|Default|SetvelocityOutput (* (* (+ (Math|Vector|GetForwardVector (Variables|Default|GetBox)) (Variables|Default|GetsteeringVector)) (Variables|Default|GetAccelerationForce)) (Variables|Default|Getboost))))
  (Physics|AddForce (Variables|Default|GetBox) _output_get "None" true))

(event Input|EnhancedActionEvents|EnhancedInputActionIA_Look
  (params (ActionValue :type Vector%202D%20Structure) (ElapsedSeconds :type Float%20%28double-precision%29) (TriggeredSeconds :type Float%20%28double-precision%29) (InputAction :type Input%20Action%20Object%20Reference :default "/Game/CarRestore/VelocityVenom2/Blueprints/VV_Pawn/Input/IA_Look.IA_Look"))
  (bind (_x _y) (Math|Vector2D|BreakVector2D ActionValue))
  ;[1 1 1] IA_Look
  (Transformation|AddRelativeRotation (Variables|Default|GetSpringArm) (Math|Rotator|MakeRotator 0.0 _y _x) false false))

(event Input|EnhancedActionEvents|EnhancedInputActionIA_Boost
  (params (ActionValue :type Boolean) (ElapsedSeconds :type Float%20%28double-precision%29) (TriggeredSeconds :type Float%20%28double-precision%29) (InputAction :type Input%20Action%20Object%20Reference :default "/Game/CarRestore/VelocityVenom2/Blueprints/VV_Pawn/Input/IA_Boost.IA_Boost"))
  ;[1 1 1] IA_Boost
  (:Triggered
    (Variables|Default|Setboost 2.0))
  (:Completed
    (Variables|Default|Setboost 1.0)))

(event Input|EnhancedActionEvents|EnhancedInputActionIA_Steer
  (params (ActionValue :type Float%20%28double-precision%29) (ElapsedSeconds :type Float%20%28double-precision%29) (TriggeredSeconds :type Float%20%28double-precision%29) (InputAction :type Input%20Action%20Object%20Reference :default "/Game/CarRestore/VelocityVenom2/Blueprints/VV_Pawn/Input/IA_Steer.IA_Steer"))
  (bind _box (Variables|Default|GetBox))
  (Class|PrimitiveComponent|AddTorqueinRadians (Variables|Default|GetBox) (Math|Vector|MakeVector 0.0 0.0 (* ActionValue 2.0)) "None" true)
  (Physics|AddForce _box (* (* (Math|Vector|GetRightVector _box) "") 1.5e+03) "None" true))

(event Input|EnhancedActionEvents|EnhancedInputActionIA_Break
  (params (ActionValue :type Boolean) (ElapsedSeconds :type Float%20%28double-precision%29) (TriggeredSeconds :type Float%20%28double-precision%29) (InputAction :type Input%20Action%20Object%20Reference :default "/Game/CarRestore/VelocityVenom2/Blueprints/VV_Pawn/Input/IA_Break.IA_Break"))
  (bind _box (Variables|Default|GetBox))
  (if (> ElapsedSeconds 2.0)
    (Physics|AddForce (Variables|Default|GetBox) (* (* (* (Math|Vector|GetForwardVector (Variables|Default|GetBox)) -1.0) (Variables|Default|GetAccelerationForce)) 0.5) "None" true)
    (else
      (bind _returnvalue (Physics|GetPhysicsLinearVelocity _box "None"))
      (Physics|SetPhysicsLinearVelocity _box (- _returnvalue (* _returnvalue 0.03)) false "None"))))

(event EventBeginPlay
  (CallFunction|Setup))

(event EventTick
  (params (DeltaSeconds :type Float%20%28single-precision%29))
  ;[1 1 1] tick Mewheels meshes
)

(event Input|KeyboardEvents|E
  (params (Key :type Key%20Structure))
  (bind _box (Variables|Default|GetBox))
  ;[1 1 1] temporary reset vehicle
  (:Pressed
    (Transformation|AddWorldOffset _box "0.000000,0.000000,300.000000" false false)
    (Transformation|SetWorldRotation _box (Math|Rotator|MakeRotator 0.0 0.0 0.0) false false)))

(fn ConstructionScript)