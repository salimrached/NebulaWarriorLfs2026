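; VV_Pawn is a drivable vehicle pawn built from a physics-simulated Box body and sphere wheels.
; Enhanced Input drives the Box with acceleration-mode forces and boost, damps velocity to brake before reversing on a long hold, and steers through angular velocity.
; Each tick, four visual wheel meshes copy sphere locations and map sphere pitch to roll.
; The E key briefly disables physics to reset rotation, and look input turns the spring arm.
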(event Custom|Setup
  (CallFunction|AddMappingInput))

(event Custom|addMappingInput
  ;[1 1 1] Add Mapping Input
  (Input|SetInputModeGameOnly (Game|GetPlayerController 0) false)
  (bind _asplayer_controller (Utilities|Casting|CastToPlayerController (Pawn|GetController)))
  (Utilities|IsValid (PlayerController|LocalPlayerSubsystems|GetEnhancedInputLocalPlayerSubsystem _asplayer_controller)
    (:Is%20Valid
      (Input|AddMappingContext (PlayerController|LocalPlayerSubsystems|GetEnhancedInputLocalPlayerSubsystem _asplayer_controller) "/Game/CarRestore/VelocityVenom2/Blueprints/VV_Pawn/Input/MC_VVPawn.MC_VVPawn" 0 "(bIgnoreAllPressedKeysUntilRelease=True,bForceImmediately=False,bNotifyUserSettings=False)"))))

(event Custom|zeroOut
  (bind _box (Variables|Default|GetBox))
  ;[1 1 1] temporary reset vehicle
  (Class|PrimitiveComponent|SetAllPhysicsLinearVelocity _box "0, 0, 0" false)
  (Class|PrimitiveComponent|SetAllPhysicsAngularVelocityinDegrees _box (Math|Vector|MakeVector 0.0 0.0 0.0) false))

(event Input|EnhancedActionEvents|EnhancedInputActionIA_Accelerate
  (params (ActionValue :type Boolean) (ElapsedSeconds :type Float%20%28double-precision%29) (TriggeredSeconds :type Float%20%28double-precision%29) (InputAction :type Input%20Action%20Object%20Reference :default "/Game/CarRestore/VelocityVenom2/Blueprints/VV_Pawn/Input/IA_Accelerate.IA_Accelerate"))
  (Physics|AddForce (Variables|Default|GetBox) (* (* (Math|Vector|GetForwardVector (Variables|Default|GetBox)) (Variables|Default|GetAccelerationForce)) (Variables|Default|Getboost)) "None" true))

(event Input|EnhancedActionEvents|EnhancedInputActionIA_Look
  (params (ActionValue :type Vector%202D%20Structure) (ElapsedSeconds :type Float%20%28double-precision%29) (TriggeredSeconds :type Float%20%28double-precision%29) (InputAction :type Input%20Action%20Object%20Reference :default "/Game/CarRestore/VelocityVenom2/Blueprints/VV_Pawn/Input/IA_Look.IA_Look"))
  (bind (_x _y) (Math|Vector2D|BreakVector2D ActionValue))
  ;[1 1 1] IA_Look
  (Transformation|AddRelativeRotation (Variables|Default|GetSpringArm) (Math|Rotator|MakeRotator 0.0 _y _x) false false))

(event Input|EnhancedActionEvents|EnhancedInputActionIA_Boost
  (params (ActionValue :type Boolean) (ElapsedSeconds :type Float%20%28double-precision%29) (TriggeredSeconds :type Float%20%28double-precision%29) (InputAction :type Input%20Action%20Object%20Reference :default "/Game/CarRestore/VelocityVenom2/Blueprints/VV_Pawn/Input/IA_Boost.IA_Boost"))
  ;[1 1 1] IA_Boost
  (:Triggered
    (Variables|Default|Setboost 2.0))
  (:Completed
    (Variables|Default|Setboost 1.0)))

(event Input|EnhancedActionEvents|EnhancedInputActionIA_Steer
  (params (ActionValue :type Float%20%28double-precision%29) (ElapsedSeconds :type Float%20%28double-precision%29) (TriggeredSeconds :type Float%20%28double-precision%29) (InputAction :type Input%20Action%20Object%20Reference :default "/Game/CarRestore/VelocityVenom2/Blueprints/VV_Pawn/Input/IA_Steer.IA_Steer"))
  (bind _box (Variables|Default|GetBox))
  (:Triggered
    (Variables|Default|SetsteerForce (- (Variables|Default|GetsteerForce) 0.1))
    (Class|PrimitiveComponent|SetPhysicsAngularVelocityinDegrees _box (Math|Vector|MakeVector 0.0 0.0 (* (* ActionValue TriggeredSeconds) (Variables|Default|GetsteerForce))) true "None")
    (Class|PrimitiveComponent|SetPhysicsMaxAngularVelocityinDegrees _box 9e+01 false "None")
    (if (< (Variables|Default|GetsteerForce) 5.0)
      (Variables|Default|SetsteerForce 5.0)))
  (:Canceled
    (Variables|Default|SetsteerForce 1e+01)))

(event Input|EnhancedActionEvents|EnhancedInputActionIA_Break
  (params (ActionValue :type Boolean) (ElapsedSeconds :type Float%20%28double-precision%29) (TriggeredSeconds :type Float%20%28double-precision%29) (InputAction :type Input%20Action%20Object%20Reference :default "/Game/CarRestore/VelocityVenom2/Blueprints/VV_Pawn/Input/IA_Break.IA_Break"))
  (bind _box (Variables|Default|GetBox))
  (if (> ElapsedSeconds 2.0)
    (Physics|AddForce (Variables|Default|GetBox) (* (* (* (Math|Vector|GetForwardVector (Variables|Default|GetBox)) -1.0) (Variables|Default|GetAccelerationForce)) 0.5) "None" true)
    (else
      (bind _returnvalue (Physics|GetPhysicsLinearVelocity _box "None"))
      (Physics|SetPhysicsLinearVelocity _box (- _returnvalue (* _returnvalue 0.03)) false "None"))))

(event EventBeginPlay
  (CallFunction|Setup))

(event EventTick
  (params (DeltaSeconds :type Float%20%28single-precision%29))
  ;[1 1 1] tick Mewheels meshes
  (CallFunction|WheelsMesh))

(event Input|KeyboardEvents|E
  (params (Key :type Key%20Structure :default "None"))
  (:Pressed
    (Physics|SetSimulatePhysics (Variables|Default|GetBox) false)
    (Transformation|SetActorRotation "0, 0, 0")
    (Utilities|FlowControl|Delay 0.4)
    (Physics|SetSimulatePhysics (Variables|Default|GetBox) true)))

(fn ConstructionScript)

(event Custom|WheelsMesh
  (bind _staticmesh (Variables|Default|GetStaticMesh))
  (bind _sphere3 (Variables|Default|GetSphere3))
  (bind _staticmesh1 (Variables|Default|GetStaticMesh1))
  (bind _sphere2 (Variables|Default|GetSphere2))
  (bind _staticmesh2 (Variables|Default|GetStaticMesh2))
  (bind _sphere (Variables|Default|GetSphere))
  (bind _staticmesh3 (Variables|Default|GetStaticMesh3))
  (bind _sphere1 (Variables|Default|GetSphere1))
  (Transformation|SetRelativeRotation _staticmesh (Math|Rotator|MakeRotator (.pitch (Variables|/Script/Engine.SceneComponent|GetRelativeRotation _sphere3)) 0.0 9e+01) false false)
  (Transformation|SetWorldLocation _staticmesh (Transformation|GetWorldLocation _sphere3) false false)
  (Transformation|SetRelativeRotation _staticmesh1 (Math|Rotator|MakeRotator (.pitch (Variables|/Script/Engine.SceneComponent|GetRelativeRotation _sphere2)) 0.0 9e+01) false false)
  (Transformation|SetWorldLocation _staticmesh1 (Transformation|GetWorldLocation _sphere2) false false)
  (Transformation|SetRelativeRotation _staticmesh2 (Math|Rotator|MakeRotator (.pitch (Variables|/Script/Engine.SceneComponent|GetRelativeRotation _sphere)) 0.0 9e+01) false false)
  (Transformation|SetWorldLocation _staticmesh2 (Transformation|GetWorldLocation _sphere) false false)
  (Transformation|SetRelativeRotation _staticmesh3 (Math|Rotator|MakeRotator (.pitch (Variables|/Script/Engine.SceneComponent|GetRelativeRotation _sphere1)) 0.0 9e+01) false false)
  (Transformation|SetWorldLocation _staticmesh3 (Transformation|GetWorldLocation _sphere1) false false))